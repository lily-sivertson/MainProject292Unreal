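; Player character Blueprint that handles third-person movement, camera look and a walk/run toggle through Enhanced Input.
; BeginPlay adds the player mapping context, and look input rotates the CameraBoom directly through relative rotation.
; Move input follows the boom's yaw and turns the mesh to match it with a -90 degree offset.
; The speed toggle flips ShouldRun, switches MaxWalkSpeed and prints debug text.
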(event Input|EnhancedActionEvents|EnhancedInputActionIA_Move
  (params (ActionValue :type Vector%202D%20Structure) (ElapsedSeconds :type Float%20%28double-precision%29) (TriggeredSeconds :type Float%20%28double-precision%29) (InputAction :type Input%20Action%20Object%20Reference :default "/Game/Charcter/Inputs/Actions/IA_Move.IA_Move"))
  (bind _cameraboom (Variables|Default|GetCameraBoom))
  (bind _relativerotation (Variables|/Script/Engine.SceneComponent|GetRelativeRotation _cameraboom))
  (:Triggered
    ;[1 1 1] Handles player movement in all directions
    (Pawn|Input|AddMovementInput (Math|Vector|GetForwardVector (Math|Rotator|MakeRotator (.roll _relativerotation) 0.0 (.yaw _relativerotation))) (.y ActionValue) false)
    (Pawn|Input|AddMovementInput (Math|Vector|GetRightVector (Math|Rotator|MakeRotator 0.0 0.0 (.yaw (Variables|/Script/Engine.SceneComponent|GetRelativeRotation (Variables|Default|GetCameraBoom))))) (.x ActionValue) false)
    (Transformation|SetRelativeRotation (Variables|Character|GetMesh) (Math|Rotator|MakeRotator 0.0 0.0 (+ (.yaw (Class|SpringArmComponent|GetTargetRotation (Variables|Default|GetCameraBoom))) -9e+01)) false false)))

(event Input|EnhancedActionEvents|EnhancedInputActionIA_Look
  (params (ActionValue :type Vector%202D%20Structure) (ElapsedSeconds :type Float%20%28double-precision%29) (TriggeredSeconds :type Float%20%28double-precision%29) (InputAction :type Input%20Action%20Object%20Reference :default "/Game/Charcter/Inputs/Actions/IA_Look.IA_Look"))
  ;[1 1 1] Controls the camera
  (:Triggered
    (Transformation|AddRelativeRotation (Variables|Default|GetCameraBoom) (Math|Rotator|MakeRotator 0.0 (.y ActionValue) (.x ActionValue)) false false)))

(event Input|EnhancedActionEvents|EnhancedInputActionIA_ToggleSpeed
  (params (ActionValue :type Boolean) (ElapsedSeconds :type Float%20%28double-precision%29) (TriggeredSeconds :type Float%20%28double-precision%29) (InputAction :type Input%20Action%20Object%20Reference :default "/Game/Charcter/Inputs/Actions/IA_ToggleSpeed.IA_ToggleSpeed"))
  ;[1 1 1] toggles player between running and walking
  (:Started
    (if (Variables|Default|GetShouldRun?)
      (Development|PrintString "should walk")
      (Variables|Default|SetShouldRun? false)
      (Variables|/Script/Engine.CharacterMovementComponent|SetMaxWalkSpeed (Variables|Character|GetCharacterMovement) 3e+02)
      (else
        (Development|PrintString "Should run")
        (Variables|Default|SetShouldRun? true)
        (Variables|/Script/Engine.CharacterMovementComponent|SetMaxWalkSpeed (Variables|Character|GetCharacterMovement) 5e+02)))))

(event EventBeginPlay
  ;[1 1 1] input mappping
  (bind _asplayer_controller (Utilities|Casting|CastToPlayerController (Pawn|GetController)))
  (Development|PrintString "yayy")
  (Utilities|IsValid (PlayerController|LocalPlayerSubsystems|GetEnhancedInputLocalPlayerSubsystem _asplayer_controller)
    (:Is%20Valid
      (Input|AddMappingContext (PlayerController|LocalPlayerSubsystems|GetEnhancedInputLocalPlayerSubsystem _asplayer_controller) "/Game/Charcter/Inputs/IMC_Player.IMC_Player" 0 "(bIgnoreAllPressedKeysUntilRelease=True,bForceImmediately=False,bNotifyUserSettings=False)"))))

(event Collision|EventActorBeginOverlap
  (params (OtherActor :type Actor%20Object%20Reference)))

(event EventTick
  (params (DeltaSeconds :type Float%20%28single-precision%29)))

(fn ConstructionScript)