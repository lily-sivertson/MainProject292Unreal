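; BPC_InteractComponent is an actor component that controls the visibility of an interaction tooltip on its owning actor.
; On BeginPlay it finds and caches the owner's WidgetComponent and hides it.
; ToggleTooltip shows or hides that widget according to whether the player is looking at it, and EndOverlapped hides it.
; The component does no detection itself, relying on outside callers to fire these events.
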(event Custom|EndOverlapped
  (Rendering|SetVisibility (Variables|Default|GetWidget) false false))

(event Custom|ToggleTooltip
  (params (PlayerLookingAt? :type Boolean))
  (bind _widget (Variables|Default|GetWidget))
  (if PlayerLookingAt?
    (Rendering|SetVisibility _widget true false)
    (else
      (Rendering|SetVisibility _widget false false))))

(event EventTick
  (params (DeltaSeconds :type Float%20%28single-precision%29)))

(event EventBeginPlay
  (bind _output_get (Variables|Default|SetWidget (Actor|GetComponentbyClass (Components|GetOwner) "/Script/UMG.WidgetComponent")))
  (Rendering|SetVisibility _output_get false false))