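; BP_OakTree is a harvestable oak tree that yields wood when its health runs out.
; On BeginPlay it hands its Healthbar to the BPC_Health component as the health widget.
; When health is depleted it looks up the Wood row in DT_Inventory, adds a random quantity to the game instance inventory, then destroys itself.
; A debug print notes that it should become a stump, but no stump is spawned.
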(event OnHealthDepleted(BPC_Health)
  (Development|PrintString "I should be a stump")
  (bind _asbp_gameinstance (Utilities|Casting|CastToBP_GAMEINSTANCE (Game|GetGameInstance)))
  (bind _returnvalue (Utilities|GetDataTableRow "/Game/ThirdPerson/Blueprints/Inventory/DT_Inventory.DT_Inventory" "Wood")
    (:then
      (Default|AddtoInv _asbp_gameinstance _returnvalue (Math|Random|RandomIntegerinRange 12 16))
      (Actor|DestroyActor))))

(event EventBeginPlay
  (Variables|/Game/Components/BPC_Health.BPC_Health_C|SetHealthWidget (Variables|Default|GetBPC_Health) (Variables|Default|GetHealthbar)))

(event Collision|EventActorBeginOverlap
  (params (OtherActor :type Actor%20Object%20Reference)))

(event EventTick
  (params (DeltaSeconds :type Float%20%28single-precision%29)))

(fn ConstructionScript)