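; BP_GiftBox is an interactable gift box that grants the player 15 carrot seeds once.
; It hands its widget to an interact component and reacts to that component's interacted event.
; On interaction it shows a WB_Dialogue message, adds the CarrotSeed row from DT_Inventory to the game instance inventory, pauses the game with the dialogue, and destroys itself.
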(event InteractedEvent(BPC_InteractComponent)
  (bind _returnvalue (UserInterface|CreateWidget "/Game/UI/WB_Dialogue.WB_Dialogue_C" (Game|GetPlayerController 0)))
  (UserInterface|Viewport|AddtoViewport _returnvalue 0)
  (Variables|/Script/UMG.TextBlock|SetText (Variables|/Game/UI/WB_Dialogue.WB_Dialogue_C|GetDialogue _returnvalue) "You Have receicved 15 Carrot Seeds!")
  (bind _asbp_gameinstance (Utilities|Casting|CastToBP_GAMEINSTANCE (Game|GetGameInstance)))
  (bind _returnvalue_2 (Utilities|GetDataTableRow "/Game/ThirdPerson/Blueprints/Inventory/DT_Inventory.DT_Inventory" "CarrotSeed")
    (:then
      (Default|AddtoInv _asbp_gameinstance _returnvalue_2 15)
      (Default|PauseGame _asbp_gameinstance _returnvalue)
      (Actor|DestroyActor self))))

(event EventBeginPlay
  (Variables|/Game/Blueprints/BPC_InteractComponent.BPC_InteractComponent_C|SetWidget (Variables|Default|GetBPC_InteractComponent) (Variables|Default|GetWidget)))

(event Collision|EventActorBeginOverlap
  (params (OtherActor :type Actor%20Object%20Reference)))

(event EventTick
  (params (DeltaSeconds :type Float%20%28single-precision%29)))

(fn ConstructionScript)