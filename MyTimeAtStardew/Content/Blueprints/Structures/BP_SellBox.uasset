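; BP_SellBox is an interactable structure that opens a selling UI for the player.
; On BeginPlay it hands its Widget to the interact component, presumably as the interaction prompt.
; When interacted with, it creates a WB_SellBox widget, loads the bag into it, adds it to the viewport and pauses the game through BP_GAMEINSTANCE.
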(event InteractedEvent(BPC_InteractComponent)
  (bind _asbp_gameinstance (Utilities|Casting|CastToBP_GAMEINSTANCE (Game|GetGameInstance)))
  (bind _returnvalue (UserInterface|CreateWidget "/Game/UI/WB_SellBox.WB_SellBox_C" (Game|GetPlayerController 0)))
  (Default|LoadBag _returnvalue)
  (UserInterface|Viewport|AddtoViewport _returnvalue 0)
  (Default|PauseGame _asbp_gameinstance _returnvalue))

(event EventBeginPlay
  (Variables|/Game/Blueprints/BPC_InteractComponent.BPC_InteractComponent_C|SetWidget (Variables|Default|GetBPC_InteractComponent) (Variables|Default|GetWidget)))

(event Collision|EventActorBeginOverlap
  (params (OtherActor :type Actor%20Object%20Reference)))

(event EventTick
  (params (DeltaSeconds :type Float%20%28single-precision%29)))

(fn ConstructionScript)