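; BP_HouseDoor is an interactable door that opens the Farm level when the player interacts with it.
; The Door component's overlap events forward to BPC_InteractComponent, which is given the Interact widget and reset to its non-overlapped state on BeginPlay.
; The component's InteractedEvent triggers the level change through an object reference.
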(event OnComponentBeginOverlap(Door)
  (params (OverlappedComponent :type Primitive%20Component%20Object%20Reference) (OtherActor :type Actor%20Object%20Reference) (OtherComp :type Primitive%20Component%20Object%20Reference) (OtherBodyIndex :type Integer) (bFromSweep :type Boolean) (SweepResult :type Hit%20Result%20Structure%20%28by%20ref%29))
  (Default|Overlapped (Variables|Default|GetBPC_InteractComponent) OtherComp))

(event OnComponentEndOverlap(Door)
  (params (OverlappedComponent :type Primitive%20Component%20Object%20Reference) (OtherActor :type Actor%20Object%20Reference) (OtherComp :type Primitive%20Component%20Object%20Reference) (OtherBodyIndex :type Integer))
  (Default|EndOverlapped (Variables|Default|GetBPC_InteractComponent)))

(event InteractedEvent(BPC_InteractComponent)
  (Game|OpenLevel(byObjectReference) "/Game/Scenes/Farm.Farm"))

(event EventBeginPlay
  (bind _bpc_interactcomponent (Variables|Default|GetBPC_InteractComponent))
  (Variables|/Game/Blueprints/BPC_InteractComponent.BPC_InteractComponent_C|SetWidget _bpc_interactcomponent (Variables|Default|GetInteract))
  (Default|EndOverlapped _bpc_interactcomponent))

(fn ConstructionScript)