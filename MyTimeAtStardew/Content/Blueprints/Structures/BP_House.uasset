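; BP_House is an interactable house structure that moves the player when used.
; Its BPC_InteractComponent event casts the player character to BP_ThirdPersonCharacter and sets it to a hardcoded location, with no level change.
; Disconnected leftover logic would write the current level name to a BP_GAMESAVETEMP save, creating one if needed, then open the FarmHouse level.
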(event InteractedEvent(BPC_InteractComponent)
  (bind _asbp_third_person_character (Utilities|Casting|CastToBP_ThirdPersonCharacter (Game|GetPlayerCharacter 0)))
  (Transformation|SetActorLocation _asbp_third_person_character "-300.000000,250.000000,-1100.000000" false false))

(fn ConstructionScript)