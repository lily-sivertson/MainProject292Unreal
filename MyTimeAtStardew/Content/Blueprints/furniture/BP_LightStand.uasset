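; BP_LightStand is a furniture light stand that can be switched on and off through interaction.
; On BeginPlay it hands its Widget to the BPC interact component.
; Each InteractedEvent from that component flips the LightON flag and sets the PointLight's visibility to match.
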(event InteractedEvent(BPC_InteractComponent)
  (if (Variables|Default|GetLightON?)
    (Variables|Default|SetLightON? false)
    (Rendering|SetVisibility (Variables|Default|GetPointLight) false false)
    (else
      (Variables|Default|SetLightON? true)
      (Rendering|SetVisibility (Variables|Default|GetPointLight) true false))))

(event EventBeginPlay
  (Variables|/Game/Blueprints/BPC_InteractComponent.BPC_InteractComponent_C|SetWidget (Variables|Default|GetBPC_InteractComponent) (Variables|Default|GetWidget)))

(event Collision|EventActorBeginOverlap
  (params (OtherActor :type Actor%20Object%20Reference)))

(event EventTick
  (params (DeltaSeconds :type Float%20%28single-precision%29)))

(fn ConstructionScript)