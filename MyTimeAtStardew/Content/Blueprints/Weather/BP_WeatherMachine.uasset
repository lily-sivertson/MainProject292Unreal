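; Weather controller actor that applies the current day's weather to the level's rain, fog, clouds and sun.
; On BeginPlay it registers itself with BP_GAMEINSTANCE and calls SetWeather, which looks up that instance's WeatherToday enum name as a DT_Weather row.
; The row toggles the Rain and Cloud actors and sets fog density and sun color.
; Rows with sound enabled also spawn audio attached to the player character's mesh.
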(event Custom|SetWeather
  (bind _rain (Variables|Default|GetRain))
  (bind _rain_2 (Variables|Default|GetRain))
  (bind _asbp_gameinstance (Utilities|Casting|CastToBP_GAMEINSTANCE (Game|GetGameInstance)))
  (bind _output_get (Variables|Default|SetWeather%20Today (Variables|/Game/Blueprints/BP_GAMEINSTANCE.BP_GAMEINSTANCE_C|GetWeatherToday _asbp_gameinstance)))
  (bind _returnvalue (Utilities|GetDataTableRow "/Game/Blueprints/Weather/DT_Weather.DT_Weather" (Utilities|String|StringToName (Utilities|String|EnumtoString _output_get)))
    (:then
      (if (.raining? _returnvalue)
        (Components|Activation|Activate (Variables|/Script/Engine.Actor|GetRootComponent _rain_2) false)
        (Rendering|SetActorHiddenInGame _rain_2 false)
        (else
          (Components|Activation|Deactivate (Variables|/Script/Engine.Actor|GetRootComponent _rain))
          (Rendering|SetActorHiddenInGame _rain true)))
      (Class|ExponentialHeightFogComponent|SetFogDensity (Variables|/Script/Engine.ExponentialHeightFog|GetComponent (Variables|Default|GetHeightFog)) (.fogdensity _returnvalue))
      (if (.cloud? _returnvalue)
        (Rendering|SetActorHiddenInGame (Variables|Default|Getcloud) false)
        (else
          (Rendering|SetActorHiddenInGame (Variables|Default|Getcloud) true)))
      (if (.sounds? _returnvalue)
        (bind _asbp_third_person_character (Utilities|Casting|CastToBP_ThirdPersonCharacter (Game|GetPlayerCharacter 0)))
        (Audio|SpawnSoundAttached (Utilities|ResolveSoftReference (.audio _returnvalue)) (Variables|/Script/Engine.Character|GetMesh _asbp_third_person_character) "None" "0, 0, 0" "0, 0, 0" "KeepRelativeOffset" true 1.0 1.0 0.0 0 0))
      (Rendering|Components|Light|SetLightColor (Variables|/Script/Engine.Light|GetLightComponent (Variables|Default|GetSun)) (Math|Conversions|ToLinearColor(Color) (.suncolor _returnvalue)) true))))

(event EventBeginPlay
  (bind _asbp_gameinstance (Utilities|Casting|CastToBP_GAMEINSTANCE (Game|GetGameInstance)))
  (Variables|/Game/Blueprints/BP_GAMEINSTANCE.BP_GAMEINSTANCE_C|SetWeatherMachine _asbp_gameinstance self)
  (CallFunction|SetWeather))

(fn ConstructionScript)