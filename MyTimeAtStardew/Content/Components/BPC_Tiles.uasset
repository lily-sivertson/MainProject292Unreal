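; BPC_Tiles is an actor component meant for dirt and sand tiles that holds logic for tilling them.
; On BeginPlay it casts its owner to BP_DirtTile, falling back to BP_Sand, and caches the reference.
; An unconnected chain would mark a tillable, untilled tile as tilled and apply TilledMat to its static mesh, but nothing triggers it.
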(event EventBeginPlay
  (bind _returnvalue (Components|GetOwner))
  (bind _asbp_dirt_tile (Utilities|Casting|CastToBP_DirtTile _returnvalue)
    (:then
      (Variables|Default|SetDirtTile _asbp_dirt_tile))
    (:CastFailed
      (bind _asbp_sand (Utilities|Casting|CastToBP_Sand _returnvalue))
      (Variables|Default|SetSandTile _asbp_sand))))

(event EventTick
  (params (DeltaSeconds :type Float%20%28single-precision%29)))